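; Player controller for the 3D nonogram game that owns the top-level UI for the main menu, solving and editor modes.
; On BeginPlay it loads saved data, then binds to the game instance's mode change event and shows the main menu.
; Each mode change removes existing widgets and creates the matching one, passing the pawn's Nonogram to solving and editor screens.
; The menu uses UI-only input, while both puzzle modes use game-and-UI input with a visible cursor.
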(event Custom|OnGameModeChanged
  (params (NewMode :type EGameMode%20Enum :default "MainMenu"))
  (CallFunction|RemoveAllwidgetsfromViewport)
  (switch Utilities|FlowControl|Switch|SwitchonEGameMode NewMode
    (:MainMenu
      (CallFunction|AddmainMenuWidgettoViewPort))
    (:Solving
      (bind _returnvalue (UserInterface|CreateWidget "/Game/Nonogram3D/Blueprints/UI/WBP_NonogramSolving.WBP_NonogramSolving_C" self (Variables|/Script/Nonogram3D.N3DPawn|GetNonogram (.AsN3DPawn (Utilities|Casting|CastToN3DPawn (Pawn|GetControlledPawn))))))
      (bind _output_get (Variables|UI|SetNonogramSolvingWidget _returnvalue))
      (UserInterface|Viewport|AddtoViewport _output_get 0)
      (Input|SetInputModeGameandUI self 0 "DoNotLock" false false :!label _label)
      (Variables|Default|SetbShowMouseCursor true))
    (:Editor
      (bind _returnvalue_2 (UserInterface|CreateWidget "/Game/Nonogram3D/Blueprints/UI/WBP_NonogramEditor.WBP_NonogramEditor_C" self (Variables|/Script/Nonogram3D.N3DPawn|GetNonogram (.AsN3DPawn (Utilities|Casting|CastToN3DPawn (Pawn|GetControlledPawn))))))
      (bind _output_get_2 (Variables|UI|SetNonogramEditorWidget _returnvalue_2))
      (UserInterface|Viewport|AddtoViewport _output_get_2 0)
      (goto _label))))

(event Custom|SaveDataLoaded
  (params (bSuccess :type Boolean))
  (if bSuccess ; TODO: Show some error, when it goes horribly wrong
    (bind _asn3dgame_instance (Utilities|Casting|CastToN3DGameInstance (Game|GetGameInstance)))
    (EventDispatchers|BindEventtoOnModeChanged _asn3dgame_instance (EventDispatchers|CreateEvent :!event Custom|OnGameModeChanged))
    (CallFunction|AddmainMenuWidgettoViewPort)))

(event EventBeginPlay
  (Class|N3DSaveSubsystem|LoadSavedData (Subsystems|GetN3DSaveSubsystem) (EventDispatchers|CreateEvent :!event Custom|SaveDataLoaded)))

(fn ConstructionScript)

(fn AddmainMenuWidgettoViewPort
  (bind _self self)
  (bind _returnvalue (UserInterface|CreateWidget "/Game/Nonogram3D/Blueprints/UI/WBP_MainMenu.WBP_MainMenu_C" _self _self))
  (bind _output_get (Variables|UI|SetMainMenuWidget _returnvalue))
  (UserInterface|Viewport|AddtoViewport _output_get 0)
  (Input|SetInputModeUIOnly self 0 "DoNotLock" false))

(fn RemoveAllwidgetsfromViewport
  (bind _mainmenuwidget (Variables|UI|GetMainMenuWidget)
    (:then
      (Widget|RemovefromParent _mainmenuwidget))
    (:else
      _))
  (bind _nonogrameditorwidget (Variables|UI|GetNonogramEditorWidget)
    (:then
      (Widget|RemovefromParent _nonogrameditorwidget))
    (:else
      _))
  (bind _nonogramsolvingwidget (Variables|UI|GetNonogramSolvingWidget)
    (:then
      (Widget|RemovefromParent _nonogramsolvingwidget))
    (:else)))