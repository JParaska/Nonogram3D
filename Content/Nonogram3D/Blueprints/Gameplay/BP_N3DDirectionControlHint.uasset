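; BP_N3DDirectionControlHint is an actor that shows the Q, E, A, D, S and W direction-control key hints in Nonogram3D.
; On BeginPlay it writes each key letter into its WBP_DirectionControlKey widget through the SetKeyText helper.
; Every Tick it sets the SpringArm's world rotation from the player controller's desired rotation with a -90 degree yaw offset, so the hint follows that orientation.
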(event EventBeginPlay
  (CallFunction|SetKeyText (Variables|Default|GetKeyQ) "Q")
  (CallFunction|SetKeyText (Variables|Default|GetKeyE) "E")
  (CallFunction|SetKeyText (Variables|Default|GetKeyA) "A")
  (CallFunction|SetKeyText (Variables|Default|GetKeyD) "D")
  (CallFunction|SetKeyText (Variables|Default|GetKeyS) "S")
  (CallFunction|SetKeyText (Variables|Default|GetKeyW) "W"))

(event EventTick
  (params (DeltaSeconds :type Float%20%28single-precision%29))
  (bind _returnvalue (Game|GetPlayerController 0))
  (bind _returnvalue_2 (Pawn|GetDesiredRotation _returnvalue))
  (Transformation|SetWorldRotation (Variables|Default|GetSpringArm) (Math|Rotator|MakeRotator (.roll _returnvalue_2) (.pitch _returnvalue_2) (- (.yaw _returnvalue_2) 9e+01)) false false))

(fn ConstructionScript)

(fn SetKeyText
  (params (Widget :type Widget%20Component%20Object%20Reference) (Text :type Text))
  (bind _aswbp_direction_control_key (Utilities|Casting|CastToWBP_DirectionControlKey (UserInterface|GetWidget Widget)))
  (Variables|/Script/UMG.TextBlock|SetText (Variables|/Game/Nonogram3D/Blueprints/UI/Nonogram/WBP_DirectionControlKey.WBP_DirectionControlKey_C|GetText_Key _aswbp_direction_control_key) Text))